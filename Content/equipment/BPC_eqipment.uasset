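; Equipment component on the third-person character that picks up weapons and toggles an equipment screen.
; The take input sphere-traces Pawn objects forward from the follow camera, adds a hit weapons_BP's data to the Slots array and destroys that actor.
; The equipment input creates or removes the Eqipment widget, switching input mode and disabling or restoring walking movement.
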(event Input|EnhancedActionEvents|EnhancedInputActionIa_take
  (params (ActionValue :type Boolean) (ElapsedSeconds :type Float%20%28double-precision%29) (TriggeredSeconds :type Float%20%28double-precision%29) (InputAction :type Input%20Action%20Object%20Reference :default "/Game/ThirdPerson/Input/Actions/Ia_take.Ia_take"))
  (bind _follow_camera (Variables|Default|GetFollow%20Camera))
  (bind _returnvalue (Transformation|GetWorldLocation _follow_camera))
  (:Started
    (bind (_outhit _returnvalue_2) (Collision|SphereTraceForObjects _returnvalue (+ _returnvalue (* (Math|Vector|GetForwardVector (Transformation|GetWorldRotation _follow_camera)) 1e+03)) 25.0 (Utilities|Array|MakeArray "ObjectTypeQuery3") false 0 "ForDuration"))
    (if _returnvalue_2
      (bind _asweapons_bp (Utilities|Casting|CastToweapons_BP (.HitActor (Collision|BreakHitResult _outhit))))
      (CallFunction|NewWeapon (Variables|/Game/equipment/weapons_BP.weapons_BP_C|Getdata _asweapons_bp))
      (Actor|DestroyActor _asweapons_bp)
      (Development|PrintString "i take it"))))

(event Input|EnhancedActionEvents|EnhancedInputActionIA_EQIPMENT
  (params (ActionValue :type Boolean) (ElapsedSeconds :type Float%20%28double-precision%29) (TriggeredSeconds :type Float%20%28double-precision%29) (InputAction :type Input%20Action%20Object%20Reference :default "/Game/ThirdPerson/Input/Actions/IA_EQIPMENT.IA_EQIPMENT"))
  (bind _returnvalue (Game|GetPlayerController 0))
  (:Started
    (if (not (Variables|Default|Getis%20open))
      (bind _returnvalue_2 (UserInterface|CreateWidget "/Game/equipment/UI/eqipment.eqipment_C"))
      (bind _output_get (Variables|Default|Setwidget _returnvalue_2))
      (UserInterface|Viewport|AddtoViewport _output_get 0)
      (Variables|/Script/Engine.PlayerController|SetbShowMouseCursor _returnvalue true)
      (Input|SetInputModeGameandUI _returnvalue (Variables|Default|Getwidget) "DoNotLock" true false)
      (bind _asbp_third_person_character (Utilities|Casting|CastToBP_ThirdPersonCharacter (Components|GetOwner)))
      (Pawn|Components|CharacterMovement|SetMovementMode (Variables|/Script/Engine.Character|GetCharacterMovement _asbp_third_person_character) "MOVE_None" 0)
      (Variables|Default|Setis%20open true)
      (else
        (bind _widget (Variables|Default|Getwidget)
          (:then
            (Widget|RemovefromParent _widget)
            (Variables|Default|Setwidget 0)
            (Variables|/Script/Engine.PlayerController|SetbShowMouseCursor _returnvalue true)
            (Input|SetInputModeGameOnly _returnvalue false)
            (bind _asbp_third_person_character_2 (Utilities|Casting|CastToBP_ThirdPersonCharacter (Components|GetOwner)))
            (Pawn|Components|CharacterMovement|SetMovementMode (Variables|/Script/Engine.Character|GetCharacterMovement _asbp_third_person_character_2) "MOVE_Walking" 0)
            (Variables|Default|Setis%20open false))
          (:else))))))

(event EventBeginPlay
  (bind _asbp_third_person_character (Utilities|Casting|CastToBP_ThirdPersonCharacter (Components|GetOwner)))
  (Variables|Default|SetFollow%20Camera (Variables|/Game/ThirdPerson/Blueprints/BP_ThirdPersonCharacter.BP_ThirdPersonCharacter_C|GetFollowCamera _asbp_third_person_character)))

(fn NewWeapon
  (params (NewItem :type Slots%20Of%20Equipment%20Structure%20%28by%20ref%29))
  (Utilities|Array|Add (Variables|Default|Getslots) NewItem))