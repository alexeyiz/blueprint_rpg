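; Victim character Blueprint that can take hits, die and flag itself for what appears to be a one-shot stealth takedown.
; The Oneshotstealth overlap volume shows the shadowless Domination component while the third-person player character is inside it and hides it on exit.
; Any damage plays a random reaction montage.
; The dead event waits briefly, then turns on mesh physics simulation and plays a death sound at the actor's location.
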(event OnComponentBeginOverlap(oneshotstealth)
  (params (OverlappedComponent :type Primitive%20Component%20Object%20Reference) (OtherActor :type Actor%20Object%20Reference) (OtherComp :type Primitive%20Component%20Object%20Reference) (OtherBodyIndex :type Integer) (bFromSweep :type Boolean) (SweepResult :type Hit%20Result%20Structure%20%28by%20ref%29))
  (Utilities|Casting|CastToBP_ThirdPersonCharacter OtherActor)
  (Rendering|SetVisibility (Variables|Default|Getdomination) true false))

(event OnComponentEndOverlap(oneshotstealth)
  (params (OverlappedComponent :type Primitive%20Component%20Object%20Reference) (OtherActor :type Actor%20Object%20Reference) (OtherComp :type Primitive%20Component%20Object%20Reference) (OtherBodyIndex :type Integer))
  (Utilities|Casting|CastToBP_ThirdPersonCharacter OtherActor)
  (Rendering|SetVisibility (Variables|Default|Getdomination) false false))

(event Custom|dead
  (Utilities|FlowControl|Delay 2.5)
  (Physics|SetSimulatePhysics (Variables|Character|GetMesh) true)
  (Audio|PlaySoundatLocation "/Game/music/fight/death.death" (Transformation|GetActorLocation) "0, 0, 0" 1.0 1.0 0.0 0 0 0 0))

(event EventBeginPlay
  (Rendering|SetCastShadow (Variables|Default|Getdomination) false))

(event Collision|EventActorBeginOverlap
  (params (OtherActor :type Actor%20Object%20Reference)))

(event EventTick
  (params (DeltaSeconds :type Float%20%28single-precision%29)))

(event Game|Damage|EventAnyDamage
  (params (Damage :type Float%20%28single-precision%29) (DamageType :type Damage%20Type%20Object%20Reference) (InstigatedBy :type Controller%20Object%20Reference) (DamageCauser :type Actor%20Object%20Reference))
  (Animation|PlayAnimMontage (Utilities|Array|Get(acopy) (Variables|Default|Getreaction%20montage) (Math|Random|RandomIntegerinRange 0 (- (Utilities|Array|Length (Variables|Default|Getreaction%20montage)) 1))) 1.0 "None"))

(fn ConstructionScript)