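; Combat component for BP_ThirdPersonCharacter that runs a four-step sword-and-kick montage combo from the attack input.
; Presses during an attack are buffered in SaveAttack, and the externally triggered newcombo event advances or resets the chain.
; A looping timer sphere-traces along the weapon, while a separate one-shot trace covers kicks.
; Hits on "damagable"-tagged actors apply damage, camera shake, blood and sound, with weapon hits throttled by a delayed DoOnce.
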(event Custom|Sword%20attack
  ;[1 1 1] combo fight
  ;;[1 1 1] combo
  (if (Variables|Default|GetAttack%20now)
    (Variables|Default|Setsave%20attack true)
    (else
      (Variables|Default|SetAttack%20now true)
      (switch int (Variables|Default|Getnumber%20of%20attack)
        (:0
          (CallFunction|FirstAttack))
        (:1
          (CallFunction|2Attack))
        (:2
          (CallFunction|3Attack))
        (:3
          (CallFunction|4Attack))))))

(event Custom|new%20combo
  ;[1 1 1] combo fight
  ;;[1 1 1] combo
  (if (Variables|Default|Getsave%20attack)
    (Variables|Default|Setsave%20attack false)
    (switch int (Variables|Default|Getnumber%20of%20attack)
      (:0
        (CallFunction|FirstAttack))
      (:1
        (CallFunction|2Attack))
      (:2
        (CallFunction|3Attack))
      (:3
        (CallFunction|4Attack)))
    (else
      (CallFunction|StopCombo))))

(event Custom|stoop%20trace
  ;[1 1 1] fight arms
  (Utilities|Time|ClearandInvalidateTimerbyHandle (Variables|Default|Getweaponloops)))

(event Custom|sphere%20trace
  (bind _blue_olayer (Variables|Default|Getblue%20olayer))
  (bind _top_of_hero (Variables|/Game/ThirdPerson/Blueprints/BP_ThirdPersonCharacter.BP_ThirdPersonCharacter_C|Gettop%20of%20hero _blue_olayer))
  (bind _returnvalue (Transformation|GetWorldLocation _top_of_hero))
  ;[1 1 1] foght legs
  (bind (_outhit _returnvalue_2) (Collision|SphereTraceByChannel _returnvalue _returnvalue 5e+01 "TraceTypeQuery1" false 0 "ForDuration" true "(R=1.000000,G=0.000000,B=0.000000,A=1.000000)" "(R=0.000000,G=1.000000,B=0.000000,A=1.000000)" 2.0))
  (if _returnvalue_2
    (if (Actor|ActorHasTag (.HitActor (Collision|BreakHitResult _outhit)) "damagable")
      (Game|Damage|ApplyDamage (.HitActor (Collision|BreakHitResult _outhit)) 1e+01 0 0)
      (Camera|PlayWorldCameraShake "/Game/blueprint/sword_camera_shake.sword_camera_shake_C" (.Location (Collision|BreakHitResult _outhit)) 0.0 2e+03)
      (Effects|SpawnEmitteratLocation "/Game/Realistic_Starter_VFX_Pack_Vol2/Particles/Blood/P_Blood_Splat_Cone.P_Blood_Splat_Cone" (.Location (Collision|BreakHitResult _outhit)) (Math|Rotator|MakeRotfromXY (.Normal (Collision|BreakHitResult _outhit)) (.Normal (Collision|BreakHitResult _outhit))) "0.600000,0.600000,0.600000" true "AutoRelease")
      (CallFunction|StartSound))))

(event Custom|Stop%20combo
  ;[1 1 1] combo fight
  ;;[1 1 1] combo
  (Variables|Default|SetAttack%20now false)
  (Variables|Default|Setnumber%20of%20attack 0))

(event Custom|4%20attack
  ;[1 1 1] combo fight
  (Utilities|FlowControl|DoOnce false :!label _label
    (:Completed
      (Utilities|FlowControl|Delay 0.1)
      (Animation|Montage|PlayMontage (Variables|Default|Getplayer) "/Game/Characters/demondetectiv/Animation/fight/Attack3_Montage.Attack3_Montage"
        (:then
          (Variables|Default|Setnumber%20of%20attack 4)
          (goto _label Reset))))))

(event Custom|First%20attack
  ;[1 1 1] combo fight
  ;;[1 1 1] 1 fttack
  (Utilities|FlowControl|DoOnce false :!label _label
    (:Completed
      (Utilities|FlowControl|Delay 0.1)
      (Animation|Montage|PlayMontage (Variables|Default|Getplayer) "/Game/Characters/demondetectiv/Animation/fight/Attack1_Montage.Attack1_Montage"
        (:then
          (Variables|Default|Setnumber%20of%20attack 1)
          (goto _label Reset))))))

(event Custom|weapon%20loop
  ;[1 1 1] fight arms
  (bind (_outhit _returnvalue) (Collision|SphereTraceByChannel (Transformation|GetWorldLocation (Variables|/Game/ThirdPerson/Blueprints/BP_ThirdPersonCharacter.BP_ThirdPersonCharacter_C|Gettop (Variables|Default|Getblue%20olayer))) (Transformation|GetWorldLocation (Variables|/Game/ThirdPerson/Blueprints/BP_ThirdPersonCharacter.BP_ThirdPersonCharacter_C|Getend (Variables|Default|Getblue%20olayer))) 5e+01 "TraceTypeQuery1" false 0 "ForDuration" true "(R=1.000000,G=0.000000,B=0.000000,A=1.000000)" "(R=0.000000,G=1.000000,B=0.000000,A=1.000000)" 2.0))
  (if _returnvalue
    (if (Actor|ActorHasTag (.HitActor (Collision|BreakHitResult _outhit)) "damagable")
      (Utilities|FlowControl|DoOnce false :!label _label
        (:Completed
          (Game|Damage|ApplyDamage (.HitActor (Collision|BreakHitResult _outhit)) 1e+01 0 0)
          (Camera|PlayWorldCameraShake "/Game/blueprint/sword_camera_shake.sword_camera_shake_C" (.Location (Collision|BreakHitResult _outhit)) 0.0 2e+03)
          (Effects|SpawnEmitteratLocation "/Game/Realistic_Starter_VFX_Pack_Vol2/Particles/Blood/P_Blood_Splat_Cone.P_Blood_Splat_Cone" (.Location (Collision|BreakHitResult _outhit)) (Math|Rotator|MakeRotfromXY (.Normal (Collision|BreakHitResult _outhit)) (.Normal (Collision|BreakHitResult _outhit))) "0.600000,0.600000,0.600000" true "AutoRelease")
          (CallFunction|StartSound)
          (Utilities|FlowControl|Delay 0.5)
          (goto _label Reset))))))

(event Custom|2%20attack
  ;[1 1 1] combo fight
  (Utilities|FlowControl|DoOnce false :!label _label
    (:Completed
      (Utilities|FlowControl|Delay 0.1)
      (Animation|Montage|PlayMontage (Variables|Default|Getplayer) "/Game/Characters/demondetectiv/Animation/fight/Attack2_Montage.Attack2_Montage"
        (:then
          (Variables|Default|Setnumber%20of%20attack 2)
          (goto _label Reset))))))

(event Custom|weapon%20trace
  ;[1 1 1] fight arms
  (bind _returnvalue (Utilities|Time|SetTimerbyEvent (delegate Custom|weapon%20loop) 0.05 true))
  (Variables|Default|Setweaponloops _returnvalue))

(event Custom|3%20attack
  ;[1 1 1] combo fight
  (Utilities|FlowControl|DoOnce false :!label _label
    (:Completed
      (Utilities|FlowControl|Delay 0.1)
      (Animation|Montage|PlayMontage (Variables|Default|Getplayer) "/Game/Characters/demondetectiv/Animation/fight/Kick_Montage.Kick_Montage"
        (:then
          (Variables|Default|Setnumber%20of%20attack 3)
          (goto _label Reset))))))

(event Custom|start%20sound
  (Audio|PlaySoundatLocation "/Game/music/sword_attack/battlestrike.battlestrike" (Transformation|GetActorLocation (Components|GetOwner)) "0, 0, 0" 1.0 1.0 0.0 0 0 0 0))

(event Input|EnhancedActionEvents|EnhancedInputActionIA_Attack
  (params (ActionValue :type Boolean) (ElapsedSeconds :type Float%20%28double-precision%29) (TriggeredSeconds :type Float%20%28double-precision%29) (InputAction :type Input%20Action%20Object%20Reference :default "/Game/ThirdPerson/Input/Actions/IA_Attack.IA_Attack"))
  ;[1 1 1] combo fight
  ;;[1 1 1] attack
  (:Started
    (if (Variables|Default|GetCan%20Attack)
      (CallFunction|SwordAttack))))

(event EventBeginPlay
  ;[1 1 1] combo fight
  (bind _asbp_third_person_character (Utilities|Casting|CastToBP_ThirdPersonCharacter (Components|GetOwner)))
  (Variables|Default|Setblue%20olayer _asbp_third_person_character)
  (Variables|Default|Setplayer (Variables|/Script/Engine.Character|GetMesh _asbp_third_person_character)))