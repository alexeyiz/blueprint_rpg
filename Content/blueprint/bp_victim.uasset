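; Victim character that the player can damage or finish with a stealth takedown, with an HP widget and a Domination indicator.
; Overlapping the Oneshotstealth volume toggles the indicator for the player.
; Damage plays a random reaction montage, launches it along the player's facing, and ragdolls it when the Statisic component's Damage returns true.
; Forkilling plays the paired knife victim montage, triggers delayed ragdoll death, and returns the killer's alignment location and rotation.
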(event OnComponentBeginOverlap(oneshotstealth)
  (params (OverlappedComponent :type Primitive%20Component%20Object%20Reference) (OtherActor :type Actor%20Object%20Reference) (OtherComp :type Primitive%20Component%20Object%20Reference) (OtherBodyIndex :type Integer) (bFromSweep :type Boolean) (SweepResult :type Hit%20Result%20Structure%20%28by%20ref%29))
  (Utilities|Casting|CastToBP_ThirdPersonCharacter OtherActor)
  (Rendering|SetVisibility (Variables|Default|Getdomination) true false))

(event OnComponentEndOverlap(oneshotstealth)
  (params (OverlappedComponent :type Primitive%20Component%20Object%20Reference) (OtherActor :type Actor%20Object%20Reference) (OtherComp :type Primitive%20Component%20Object%20Reference) (OtherBodyIndex :type Integer))
  (Utilities|Casting|CastToBP_ThirdPersonCharacter OtherActor)
  (Rendering|SetVisibility (Variables|Default|Getdomination) false false))

(event Custom|dead
  (Utilities|FlowControl|Delay 2.5)
  (Physics|SetSimulatePhysics (Variables|Character|GetMesh) true)
  (Audio|PlaySoundatLocation "/Game/music/fight/death.death" (Transformation|GetActorLocation) "0, 0, 0" 1.0 1.0 0.0 0 0 0 0)
  (Rendering|SetVisibility (Variables|Default|Getdomination) false false))

(event EventBeginPlay
  (Rendering|SetCastShadow (Variables|Default|Getdomination) false)
  (bind _asvictim_hp (Utilities|Casting|CastTovictim_hp (UserInterface|GetWidget (Variables|Default|Gethp))))
  (Variables|Default|SetAs%20Victim%20Hp _asvictim_hp))

(event Collision|EventActorBeginOverlap
  (params (OtherActor :type Actor%20Object%20Reference)))

(event EventTick
  (params (DeltaSeconds :type Float%20%28single-precision%29)))

(event Game|Damage|EventAnyDamage
  (params (Damage :type Float%20%28single-precision%29) (DamageType :type Damage%20Type%20Object%20Reference) (InstigatedBy :type Controller%20Object%20Reference) (DamageCauser :type Actor%20Object%20Reference))
  (Animation|PlayAnimMontage (Utilities|Array|Get(acopy) (Variables|Default|Getreaction%20montage) (Math|Random|RandomIntegerinRange 0 (- (Utilities|Array|Length (Variables|Default|Getreaction%20montage)) 1))) 1.0 "None")
  (bind _asbp_third_person_character (Utilities|Casting|CastToBP_ThirdPersonCharacter (Game|GetPlayerCharacter 0)))
  (Character|LaunchCharacter (* (Math|Vector|GetForwardVector (Transformation|GetActorRotation _asbp_third_person_character)) 7e+02) false false)
  (Audio|PlaySoundatLocation "/Game/music/fight/death.death" (Transformation|GetActorLocation) "0, 0, 0" 1.0 1.0 0.0 0 0 0 0)
  (bind _player_death (Default|Damage (Variables|Default|Getstatisic) Damage))
  (if _player_death
    (Physics|SetSimulatePhysics (Variables|Character|GetMesh) true)
    (Audio|PlaySoundatLocation "/Game/music/fight/death.death" (Transformation|GetActorLocation) "0, 0, 0" 1.0 1.0 0.0 0 0 0 0)
    (Rendering|SetVisibility (Variables|Default|Gethp) false false)))

(fn ConstructionScript)

(fn Forkilling
  (Animation|PlayAnimMontage "/Game/Characters/demondetectiv/Animation/stealth/Paired_Knife_Stealth_KidneyAndNeck_Vic_Montage.Paired_Knife_Stealth_KidneyAndNeck_Vic_Montage" 1.0 "None")
  (CallFunction|Dead)
  (Rendering|SetVisibility (Variables|Default|Getdomination) false false)
  (return (Transformation|GetWorldLocation (Variables|Default|Getmeshofkiller)) (Transformation|GetActorRotation)))